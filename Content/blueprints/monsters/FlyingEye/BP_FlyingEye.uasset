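; BP_FlyingEye is a flying eye monster that patrols back and forth along the X axis and damages actors it touches.
; Each tick steps counter S1 toward signed limit S; on reaching it, S flips and the sprite turns, so patrol length depends on frame rate.
; BoxHit overlap applies damage, launches the eye along +X and pauses patrol briefly.
; S1 is printed every unlocked tick.
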(event `self.ReceiveTick`
  (params (DeltaSeconds :type "Float (single-precision)"))
  (`self.follow`))

(event `self.BoxHit.OnComponentBeginOverlap`
  (params (OverlappedComponent :type "PrimitiveComponent Object Reference") (OtherActor :type "Actor Object Reference") (OtherComp :type "PrimitiveComponent Object Reference") (OtherBodyIndex :type Integer) (bFromSweep :type Boolean) (SweepResult :type "HitResult Structure (by ref)"))
  (`GameplayStatics.ApplyDamage` OtherActor 10.0)
  (`self.LaunchCharacter` (500.0 0.0 0.0) true)
  (set `self.isMovementLock` true)
  (`KismetSystemLibrary.Delay` 2.0)
  (set `self.isMovementLock` false))

(event `follow`
  (if (not (`self.isMovementLock`))
    (`KismetSystemLibrary.PrintString` (`KismetStringLibrary.Conv_DoubleToString` (`self.s1`)))
    (`/Engine/EditorBlueprintResources/StandardMacros.CompareFloat` (`self.s1`) (`self.s`)
      (:`>`
        (`self.AddMovementInput` (-1.0 0.0 0.0))
        (set `self.s1` (- (`self.s1`) 1.0)))
      (:`==`
        (if (> (`self.s`) 0.0)
          (set `self.s` (* (`self.s`) -1.0))
          (set `self.s1` 0.0)
          (`SceneComponent.K2_SetRelativeRotation` (`self.Sprite`) (struct :`Yaw` 180.0) false false)
          (else
            (set `self.s` (* (`self.s`) -1.0))
            (set `self.s1` 0.0)
            (`SceneComponent.K2_SetRelativeRotation` (`self.Sprite`) (struct) false false))))
      (:`<`
        (`self.AddMovementInput` (1.0 0.0 0.0))
        (set `self.s1` (+ (`self.s1`) 1.0))))))

(fn `UserConstructionScript`)